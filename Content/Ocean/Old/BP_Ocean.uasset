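; Ocean actor that configures the water surface and depth-plane materials for a selectable shader variant, from Gerstner waves to foam, SSR and cubemap options.
; The construction script creates the dynamic material instances, then pushes an eight-wave set, global wave cluster values and look settings into MPC_Ocean.
; BeginPlay repeats the parameter pushes.
; With a valid Landscape and heightmap, it also passes terrain texture, transform and modulation values to the materials.
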(event EventBeginPlay
  (CallFunction|CreateWaveSet)
  (CallFunction|SetGlobalParameters)
  (CallFunction|SetDisplayParameters))

(fn ConstructionScript
  (bind _depthplanetopside (Variables|Default|GetDepthPlaneTopside))
  (Utilities|FlowControl|Sequence
    (:then_0
      ;[1 1 1] Set the material instance
      (bind _returnvalue (Rendering|Material|CreateDynamicMaterialInstance (Variables|Default|GetOceanPlane) 0 (Utilities|Select :Index (Variables|Appearance|GetOceanShader) :NewEnumerator0 "/Game/Ocean/Materials/M_Ocean_Versions/M_Ocean_Old.M_Ocean_Old" :NewEnumerator1 "/Game/Ocean/Materials/M_Ocean_Versions/M_Ocean.M_Ocean" :NewEnumerator2 "/Game/Ocean/Materials/M_Ocean_Versions/M_Ocean_SSR.M_Ocean_SSR" :NewEnumerator3 "/Game/Ocean/Materials/M_Ocean_Versions/M_Inst_Ocean_Foam.M_Inst_Ocean_Foam" :NewEnumerator8 "/Game/Ocean/Materials/M_Ocean_Versions/M_Inst_Ocean_Foam_Cubemap.M_Inst_Ocean_Foam_Cubemap" :NewEnumerator6 "/Game/Ocean/Materials/M_Ocean_Versions/M_Inst_Ocean_SSR_Foam.M_Inst_Ocean_SSR_Foam" :NewEnumerator7 "/Game/Ocean/Materials/M_Ocean_Versions/M_Inst_Ocean_SSR_Foam_Cubemap.M_Inst_Ocean_SSR_Foam_Cubemap" :NewEnumerator4 "/Game/Ocean/Materials/M_Ocean_Versions/M_Inst_Ocean_Nogerstner.M_Inst_Ocean_Nogerstner" :NewEnumerator5 "/Game/Ocean/Materials/M_Ocean_Versions/M_Inst_Ocean_SSR_Nogerstner.M_Inst_Ocean_SSR_Nogerstner" :NewEnumerator9 "/Game/Ocean/Materials/M_Ocean_Versions/M_Inst_Ocean_Ultra.M_Inst_Ocean_Ultra" :NewEnumerator10 0) :!class /Script/Engine.PrimitiveComponent))
      (Variables|Default|SetMID_Ocean _returnvalue)
      ;[1 1 1] Setup material instance
      (switch Utilities|FlowControl|Switch|SwitchonOceanShaderEnum (Variables|Appearance|GetOceanShader)
        (:NewEnumerator0
          (bind _returnvalue_2 (Rendering|Material|CreateDynamicMaterialInstance _depthplanetopside 0 "/Game/Ocean/Materials/M_Ocean_Versions/M_Inst_Ocean_Ultra.M_Inst_Ocean_Ultra" :!class /Script/Engine.PrimitiveComponent :!label _label))
          (bind _output_get (Variables|Default|SetMID_Ocean_Depth _returnvalue_2)))
        (:NewEnumerator1
          (goto _label))
        (:NewEnumerator2
          (goto _label))
        (:NewEnumerator3
          (goto _label))
        (:NewEnumerator8
          (goto _label))
        (:NewEnumerator6
          (goto _label))
        (:NewEnumerator7
          (goto _label))
        (:NewEnumerator4
          (bind _returnvalue_3 (Rendering|Material|CreateDynamicMaterialInstance _depthplanetopside 0 "/Game/Ocean/Materials/M_Ocean_Versions/M_Inst_Ocean_Depth_Nogerstner.M_Inst_Ocean_Depth_Nogerstner" :!class /Script/Engine.PrimitiveComponent :!label _label_2))
          (Variables|Default|SetMID_Ocean_Depth _returnvalue_3))
        (:NewEnumerator5
          (goto _label_2))
        (:NewEnumerator9
          (bind _returnvalue_4 (Rendering|Material|CreateDynamicMaterialInstance _depthplanetopside 0 "/Game/Ocean/Materials/M_Ocean_Versions/M_Inst_Ocean_Depth_Ultra.M_Inst_Ocean_Depth_Ultra" :!class /Script/Engine.PrimitiveComponent))
          (Variables|Default|SetMID_Ocean_Depth _returnvalue_4))
        (:NewEnumerator10
          (goto _label)))
      (Rendering|Material|SetMaterial (Variables|Default|GetDepthPlaneUnderside) 0 _output_get))
    (:then_1
      ;[1 1 1] Set global parameters
      (CallFunction|SetGlobalParameters)
      (CallFunction|SetDisplayParameters))
    (:then_2
      ;[1 1 1] Create wave set
      (CallFunction|CreateWaveSet))))

(fn CreateWaveSet
  ;[1 1 1] Intliaze Wave set
  (Utilities|FlowControl|Sequence
    (:then_0
      (if (> (Utilities|Array|Length (Variables|OceanManager|GetWaveSetOffsetsOVerride)) 0)
        (LocalVariables|SetSetPharams (Utilities|Array|Get(acopy) (Variables|OceanManager|GetWaveSetOffsetsOVerride)))))
    (:then_1
      (Rendering|Material|SetVectorParameterValue "/Game/Ocean/Materials/MPC_Ocean.MPC_Ocean" "Set01Wave01" (Math|Color|MakeColor (.Rotation (Utilities|Struct|BreakWaveParameters (.Wave01 (Utilities|Struct|BreakWaveSet (LocalVariables|GetSetPharams))))) (.Length (Utilities|Struct|BreakWaveParameters (.Wave01 (Utilities|Struct|BreakWaveSet (LocalVariables|GetSetPharams))))) (.Amplitude (Utilities|Struct|BreakWaveParameters (.Wave01 (Utilities|Struct|BreakWaveSet (LocalVariables|GetSetPharams))))) (.Steepness (Utilities|Struct|BreakWaveParameters (.Wave01 (Utilities|Struct|BreakWaveSet (LocalVariables|GetSetPharams)))))) :!class /Script/Engine.KismetMaterialLibrary)
      (Rendering|Material|SetVectorParameterValue "/Game/Ocean/Materials/MPC_Ocean.MPC_Ocean" "Set01Wave02" (Math|Color|MakeColor (.Rotation (Utilities|Struct|BreakWaveParameters (.Wave02 (Utilities|Struct|BreakWaveSet (LocalVariables|GetSetPharams))))) (.Length (Utilities|Struct|BreakWaveParameters (.Wave02 (Utilities|Struct|BreakWaveSet (LocalVariables|GetSetPharams))))) (.Amplitude (Utilities|Struct|BreakWaveParameters (.Wave02 (Utilities|Struct|BreakWaveSet (LocalVariables|GetSetPharams))))) (.Steepness (Utilities|Struct|BreakWaveParameters (.Wave02 (Utilities|Struct|BreakWaveSet (LocalVariables|GetSetPharams)))))) :!class /Script/Engine.KismetMaterialLibrary)
      (Rendering|Material|SetVectorParameterValue "/Game/Ocean/Materials/MPC_Ocean.MPC_Ocean" "Set01Wave03" (Math|Color|MakeColor (.Rotation (Utilities|Struct|BreakWaveParameters (.Wave03 (Utilities|Struct|BreakWaveSet (LocalVariables|GetSetPharams))))) (.Length (Utilities|Struct|BreakWaveParameters (.Wave03 (Utilities|Struct|BreakWaveSet (LocalVariables|GetSetPharams))))) (.Amplitude (Utilities|Struct|BreakWaveParameters (.Wave03 (Utilities|Struct|BreakWaveSet (LocalVariables|GetSetPharams))))) (.Steepness (Utilities|Struct|BreakWaveParameters (.Wave03 (Utilities|Struct|BreakWaveSet (LocalVariables|GetSetPharams)))))) :!class /Script/Engine.KismetMaterialLibrary)
      (Rendering|Material|SetVectorParameterValue "/Game/Ocean/Materials/MPC_Ocean.MPC_Ocean" "Set01Wave04" (Math|Color|MakeColor (.Rotation (Utilities|Struct|BreakWaveParameters (.Wave04 (Utilities|Struct|BreakWaveSet (LocalVariables|GetSetPharams))))) (.Length (Utilities|Struct|BreakWaveParameters (.Wave04 (Utilities|Struct|BreakWaveSet (LocalVariables|GetSetPharams))))) (.Amplitude (Utilities|Struct|BreakWaveParameters (.Wave04 (Utilities|Struct|BreakWaveSet (LocalVariables|GetSetPharams))))) (.Steepness (Utilities|Struct|BreakWaveParameters (.Wave04 (Utilities|Struct|BreakWaveSet (LocalVariables|GetSetPharams)))))) :!class /Script/Engine.KismetMaterialLibrary)
      (Rendering|Material|SetVectorParameterValue "/Game/Ocean/Materials/MPC_Ocean.MPC_Ocean" "Set01Wave05" (Math|Color|MakeColor (.Rotation (Utilities|Struct|BreakWaveParameters (.Wave05 (Utilities|Struct|BreakWaveSet (LocalVariables|GetSetPharams))))) (.Length (Utilities|Struct|BreakWaveParameters (.Wave05 (Utilities|Struct|BreakWaveSet (LocalVariables|GetSetPharams))))) (.Amplitude (Utilities|Struct|BreakWaveParameters (.Wave05 (Utilities|Struct|BreakWaveSet (LocalVariables|GetSetPharams))))) (.Steepness (Utilities|Struct|BreakWaveParameters (.Wave05 (Utilities|Struct|BreakWaveSet (LocalVariables|GetSetPharams)))))) :!class /Script/Engine.KismetMaterialLibrary)
      (Rendering|Material|SetVectorParameterValue "/Game/Ocean/Materials/MPC_Ocean.MPC_Ocean" "Set01Wave06" (Math|Color|MakeColor (.Rotation (Utilities|Struct|BreakWaveParameters (.Wave06 (Utilities|Struct|BreakWaveSet (LocalVariables|GetSetPharams))))) (.Length (Utilities|Struct|BreakWaveParameters (.Wave06 (Utilities|Struct|BreakWaveSet (LocalVariables|GetSetPharams))))) (.Amplitude (Utilities|Struct|BreakWaveParameters (.Wave06 (Utilities|Struct|BreakWaveSet (LocalVariables|GetSetPharams))))) (.Steepness (Utilities|Struct|BreakWaveParameters (.Wave06 (Utilities|Struct|BreakWaveSet (LocalVariables|GetSetPharams)))))) :!class /Script/Engine.KismetMaterialLibrary)
      (Rendering|Material|SetVectorParameterValue "/Game/Ocean/Materials/MPC_Ocean.MPC_Ocean" "Set01Wave07" (Math|Color|MakeColor (.Rotation (Utilities|Struct|BreakWaveParameters (.Wave07 (Utilities|Struct|BreakWaveSet (LocalVariables|GetSetPharams))))) (.Length (Utilities|Struct|BreakWaveParameters (.Wave07 (Utilities|Struct|BreakWaveSet (LocalVariables|GetSetPharams))))) (.Amplitude (Utilities|Struct|BreakWaveParameters (.Wave07 (Utilities|Struct|BreakWaveSet (LocalVariables|GetSetPharams))))) (.Steepness (Utilities|Struct|BreakWaveParameters (.Wave07 (Utilities|Struct|BreakWaveSet (LocalVariables|GetSetPharams)))))) :!class /Script/Engine.KismetMaterialLibrary)
      (Rendering|Material|SetVectorParameterValue "/Game/Ocean/Materials/MPC_Ocean.MPC_Ocean" "Set01Wave08" (Math|Color|MakeColor (.Rotation (Utilities|Struct|BreakWaveParameters (.Wave08 (Utilities|Struct|BreakWaveSet (LocalVariables|GetSetPharams))))) (.Length (Utilities|Struct|BreakWaveParameters (.Wave08 (Utilities|Struct|BreakWaveSet (LocalVariables|GetSetPharams))))) (.Amplitude (Utilities|Struct|BreakWaveParameters (.Wave08 (Utilities|Struct|BreakWaveSet (LocalVariables|GetSetPharams))))) (.Steepness (Utilities|Struct|BreakWaveParameters (.Wave08 (Utilities|Struct|BreakWaveSet (LocalVariables|GetSetPharams)))))) :!class /Script/Engine.KismetMaterialLibrary))))

(fn SetDisplayParameters
  (Utilities|FlowControl|Sequence
    (:then_0
      ;[1 1 1] Base Material Properties
      (Rendering|Material|SetVectorParameterValue "/Game/Ocean/Materials/MPC_Ocean.MPC_Ocean" "BaseColorDark" (Variables|Appearance|GetBase%20Color%20Dark) :!class /Script/Engine.KismetMaterialLibrary)
      (Rendering|Material|SetVectorParameterValue "/Game/Ocean/Materials/MPC_Ocean.MPC_Ocean" "BaseColorLight" (Variables|Appearance|GetBase%20Color%20Light) :!class /Script/Engine.KismetMaterialLibrary)
      (Rendering|Material|SetScalarParameterValue "/Game/Ocean/Materials/MPC_Ocean.MPC_Ocean" "BaseColorLerp" (Variables|Appearance|GetBase%20Color%20Lerp) :!class /Script/Engine.KismetMaterialLibrary)
      (Rendering|Material|SetScalarParameterValue "/Game/Ocean/Materials/MPC_Ocean.MPC_Ocean" "BaseFresnelPower" (Variables|Appearance|GetFresnel%20Power) :!class /Script/Engine.KismetMaterialLibrary)
      (Rendering|Material|SetScalarParameterValue "/Game/Ocean/Materials/MPC_Ocean.MPC_Ocean" "BaseFresnelReflect" (Variables|Appearance|GetBase%20Fresnel%20Reflect) :!class /Script/Engine.KismetMaterialLibrary)
      (Rendering|Material|SetScalarParameterValue "/Game/Ocean/Materials/MPC_Ocean.MPC_Ocean" "Metallic" (Variables|Appearance|GetMetallic) :!class /Script/Engine.KismetMaterialLibrary)
      (Rendering|Material|SetScalarParameterValue "/Game/Ocean/Materials/MPC_Ocean.MPC_Ocean" "Roughness" (Variables|Appearance|GetRoughness) :!class /Script/Engine.KismetMaterialLibrary)
      (Rendering|Material|SetScalarParameterValue "/Game/Ocean/Materials/MPC_Ocean.MPC_Ocean" "Specular" (Variables|Appearance|GetSpecular) :!class /Script/Engine.KismetMaterialLibrary)
      (Rendering|Material|SetScalarParameterValue "/Game/Ocean/Materials/MPC_Ocean.MPC_Ocean" "TesselationMultiplier" (Variables|Appearance|GetTesselation%20Multiplier%20) :!class /Script/Engine.KismetMaterialLibrary)
      (Rendering|Material|SetVectorParameterValue "/Game/Ocean/Materials/MPC_Ocean.MPC_Ocean" "ShallowColor" (Variables|Appearance|GetShallow%20Water%20Color) :!class /Script/Engine.KismetMaterialLibrary))
    (:then_1
      ;[1 1 1] Base Extended Properties
      (Rendering|Material|SetScalarParameterValue "/Game/Ocean/Materials/MPC_Ocean.MPC_Ocean" "Opacity" (Variables|Appearance|GetOpacity) :!class /Script/Engine.KismetMaterialLibrary)
      (Rendering|Material|SetScalarParameterValue "/Game/Ocean/Materials/MPC_Ocean.MPC_Ocean" "DepthFade" (Variables|Appearance|GetBase%20Depth%20Fade) :!class /Script/Engine.KismetMaterialLibrary)
      (Rendering|Material|SetScalarParameterValue "/Game/Ocean/Materials/MPC_Ocean.MPC_Ocean" "DistortionStrength" (Variables|Appearance|GetDistortion%20Strength) :!class /Script/Engine.KismetMaterialLibrary)
      (Rendering|Material|SetScalarParameterValue "/Game/Ocean/Materials/MPC_Ocean.MPC_Ocean" "SceneColorDepthFade" (Variables|Appearance|GetScene%20Color%20Custom%20Depth) :!class /Script/Engine.KismetMaterialLibrary)
      (Rendering|Material|SetScalarParameterValue "/Game/Ocean/Materials/MPC_Ocean.MPC_Ocean" "FoamScale" (Variables|Appearance|GetFoam%20Scale) :!class /Script/Engine.KismetMaterialLibrary)
      (Rendering|Material|SetScalarParameterValue "/Game/Ocean/Materials/MPC_Ocean.MPC_Ocean" "DepthTest1" (Variables|Appearance|GetFoam%20Depth%201) :!class /Script/Engine.KismetMaterialLibrary)
      (Rendering|Material|SetScalarParameterValue "/Game/Ocean/Materials/MPC_Ocean.MPC_Ocean" "DepthTest2" (Variables|Appearance|GetFoam%20Depth%202) :!class /Script/Engine.KismetMaterialLibrary)
      (Rendering|Material|SetScalarParameterValue "/Game/Ocean/Materials/MPC_Ocean.MPC_Ocean" "FoamTimeScale" (Variables|Appearance|GetFoam%20Time%20Scale) :!class /Script/Engine.KismetMaterialLibrary)
      (Rendering|Material|SetScalarParameterValue "/Game/Ocean/Materials/MPC_Ocean.MPC_Ocean" "FoamSoftness" (Variables|Appearance|GetFoam%20Softness%201) :!class /Script/Engine.KismetMaterialLibrary)
      (Rendering|Material|SetScalarParameterValue "/Game/Ocean/Materials/MPC_Ocean.MPC_Ocean" "SceneDepthSoftness" (Variables|Appearance|GetScene%20Depth%20Softness) :!class /Script/Engine.KismetMaterialLibrary)
      (Rendering|Material|SetScalarParameterValue "/Game/Ocean/Materials/MPC_Ocean.MPC_Ocean" "BaseDepthFadeSoftness" (Variables|Appearance|GetBase%20Depth%20Fade%20Sotness) :!class /Script/Engine.KismetMaterialLibrary))
    (:then_2
      ;[1 1 1] Subsurface Scattering
      (Rendering|Material|SetVectorParameterValue "/Game/Ocean/Materials/MPC_Ocean.MPC_Ocean" "SSS_Color" (Variables|SubsurfaceScattering|GetSSS_Color) :!class /Script/Engine.KismetMaterialLibrary)
      (Rendering|Material|SetScalarParameterValue "/Game/Ocean/Materials/MPC_Ocean.MPC_Ocean" "SSS_Scale" (Variables|SubsurfaceScattering|GetSSS%20Scale) :!class /Script/Engine.KismetMaterialLibrary)
      (Rendering|Material|SetScalarParameterValue "/Game/Ocean/Materials/MPC_Ocean.MPC_Ocean" "SSS_Intensity" (Variables|SubsurfaceScattering|GetSSS_Intensity) :!class /Script/Engine.KismetMaterialLibrary)
      (Rendering|Material|SetScalarParameterValue "/Game/Ocean/Materials/MPC_Ocean.MPC_Ocean" "SSS_LightDepth" (Variables|SubsurfaceScattering|GetSSS_LightDepth) :!class /Script/Engine.KismetMaterialLibrary)
      (Rendering|Material|SetScalarParameterValue "/Game/Ocean/Materials/MPC_Ocean.MPC_Ocean" "SSS_MacroNormalStrength" (Variables|SubsurfaceScattering|GetSSS%20Macro%20Normal%20Strength) :!class /Script/Engine.KismetMaterialLibrary))
    (:then_3
      ;[1 1 1] Panning Normals
      (Rendering|Material|SetScalarParameterValue "/Game/Ocean/Materials/MPC_Ocean.MPC_Ocean" "PanWaveLerp" (Variables|PanningNormals|GetPan%20Wave%20Lerp) :!class /Script/Engine.KismetMaterialLibrary)
      (Rendering|Material|SetScalarParameterValue "/Game/Ocean/Materials/MPC_Ocean.MPC_Ocean" "PanWaveIntensity" (Variables|PanningNormals|GetPan%20Wave%20Intensity) :!class /Script/Engine.KismetMaterialLibrary)
      (Rendering|Material|SetScalarParameterValue "/Game/Ocean/Materials/MPC_Ocean.MPC_Ocean" "PanWaveTimeScale" (Variables|PanningNormals|GetPan%20Wave%20Time%20Scale) :!class /Script/Engine.KismetMaterialLibrary)
      (Rendering|Material|SetScalarParameterValue "/Game/Ocean/Materials/MPC_Ocean.MPC_Ocean" "PanWaveSize" (Variables|PanningNormals|GetPan%20Wave%20Size) :!class /Script/Engine.KismetMaterialLibrary)
      (Rendering|Material|SetVectorParameterValue "/Game/Ocean/Materials/MPC_Ocean.MPC_Ocean" "PanWave01SpeedV2" (Math|Conversions|ToLinearColor(Vector) (Variables|PanningNormals|GetPanner%2001%20Speed)) :!class /Script/Engine.KismetMaterialLibrary)
      (Rendering|Material|SetVectorParameterValue "/Game/Ocean/Materials/MPC_Ocean.MPC_Ocean" "PanWave01SpeedV2" (Math|Conversions|ToLinearColor(Vector) (Variables|PanningNormals|GetPanner%2002%20Speed)) :!class /Script/Engine.KismetMaterialLibrary)
      (Rendering|Material|SetVectorParameterValue "/Game/Ocean/Materials/MPC_Ocean.MPC_Ocean" "PanWave01SpeedV2" (Math|Conversions|ToLinearColor(Vector) (Variables|PanningNormals|GetPanner%2003%20Speed)) :!class /Script/Engine.KismetMaterialLibrary)
      ;[1 1 1] Macro Waves
      (Rendering|Material|SetScalarParameterValue "/Game/Ocean/Materials/MPC_Ocean.MPC_Ocean" "MacroScale" (Variables|PanningNormals|GetMacro%20Wave%20Scale) :!class /Script/Engine.KismetMaterialLibrary)
      (Rendering|Material|SetScalarParameterValue "/Game/Ocean/Materials/MPC_Ocean.MPC_Ocean" "MacroSpeed" (Variables|PanningNormals|GetMacro%20Wave%20Speed) :!class /Script/Engine.KismetMaterialLibrary)
      (Rendering|Material|SetScalarParameterValue "/Game/Ocean/Materials/MPC_Ocean.MPC_Ocean" "MacroAmplify" (Variables|PanningNormals|GetMacro%20Wave%20Amplify) :!class /Script/Engine.KismetMaterialLibrary))
    (:then_4
      ;[1 1 1] Detail,Medium and Far Normals
      (Rendering|Material|SetScalarParameterValue "/Game/Ocean/Materials/MPC_Ocean.MPC_Ocean" "DetailNormalScale" (Variables|Detail,MediumandFarNormals|GetDetail%20Normal%20Scale) :!class /Script/Engine.KismetMaterialLibrary)
      (Rendering|Material|SetScalarParameterValue "/Game/Ocean/Materials/MPC_Ocean.MPC_Ocean" "DetailNormalSpeed" (Variables|Detail,MediumandFarNormals|GetDetail%20Normal%20Speed) :!class /Script/Engine.KismetMaterialLibrary)
      (Rendering|Material|SetScalarParameterValue "/Game/Ocean/Materials/MPC_Ocean.MPC_Ocean" "DetailNormalStrength" (Variables|Detail,MediumandFarNormals|GetDetail%20Normal%20Strength) :!class /Script/Engine.KismetMaterialLibrary)
      (Rendering|Material|SetScalarParameterValue "/Game/Ocean/Materials/MPC_Ocean.MPC_Ocean" "MediumNormalScale" (Variables|Detail,MediumandFarNormals|GetMedium%20Normal%20Scale) :!class /Script/Engine.KismetMaterialLibrary)
      (Rendering|Material|SetScalarParameterValue "/Game/Ocean/Materials/MPC_Ocean.MPC_Ocean" "MediumNormalSpeed" (Variables|Detail,MediumandFarNormals|GetMedium%20Normal%20Speed) :!class /Script/Engine.KismetMaterialLibrary)
      (Rendering|Material|SetScalarParameterValue "/Game/Ocean/Materials/MPC_Ocean.MPC_Ocean" "MediumNormalStrength" (Variables|Detail,MediumandFarNormals|GetMedium%20Normal%20Strength) :!class /Script/Engine.KismetMaterialLibrary)
      (Rendering|Material|SetScalarParameterValue "/Game/Ocean/Materials/MPC_Ocean.MPC_Ocean" "FarNormalScale" (Variables|Detail,MediumandFarNormals|GetFar%20Normal%20Scale) :!class /Script/Engine.KismetMaterialLibrary)
      (Rendering|Material|SetScalarParameterValue "/Game/Ocean/Materials/MPC_Ocean.MPC_Ocean" "FarNormalSpeed" (Variables|Detail,MediumandFarNormals|GetFar%20Normal%20Speed) :!class /Script/Engine.KismetMaterialLibrary)
      (Rendering|Material|SetScalarParameterValue "/Game/Ocean/Materials/MPC_Ocean.MPC_Ocean" "FarNormalStrength" (Variables|Detail,MediumandFarNormals|GetFar%20Normal%20Strength) :!class /Script/Engine.KismetMaterialLibrary)
      (Rendering|Material|SetScalarParameterValue "/Game/Ocean/Materials/MPC_Ocean.MPC_Ocean" "FarNormalBlendDistance" (Variables|Detail,MediumandFarNormals|GetFar%20Normal%20Blend%20Distance) :!class /Script/Engine.KismetMaterialLibrary)
      (Rendering|Material|SetScalarParameterValue "/Game/Ocean/Materials/MPC_Ocean.MPC_Ocean" "FarNormalBlendFalloff" (Variables|Detail,MediumandFarNormals|GetFar%20Normal%20Blend%20Falloff) :!class /Script/Engine.KismetMaterialLibrary))
    (:then_5
      ;[1 1 1] Heightmap Parameters
      (Rendering|Material|SetScalarParameterValue "/Game/Ocean/Materials/MPC_Ocean.MPC_Ocean" "HeightmapDisplacement" (Variables|Heightmap|GetHeightmap%20Displacement) :!class /Script/Engine.KismetMaterialLibrary)
      (Rendering|Material|SetScalarParameterValue "/Game/Ocean/Materials/MPC_Ocean.MPC_Ocean" "HeightmapScale" (Variables|Heightmap|GetHeightmap%20Scale) :!class /Script/Engine.KismetMaterialLibrary)
      (Rendering|Material|SetScalarParameterValue "/Game/Ocean/Materials/MPC_Ocean.MPC_Ocean" "HeightmapSpeed" (Variables|Heightmap|GetHeightmap%20Speed) :!class /Script/Engine.KismetMaterialLibrary))
    (:then_6
      ;[1 1 1] Seafoam parameters
      (Rendering|Material|SetScalarParameterValue "/Game/Ocean/Materials/MPC_Ocean.MPC_Ocean" "SeafoamScale" (Variables|Seafoam|GetSeafoam%20Scale) :!class /Script/Engine.KismetMaterialLibrary)
      (Rendering|Material|SetScalarParameterValue "/Game/Ocean/Materials/MPC_Ocean.MPC_Ocean" "SeafoamSpeed" (Variables|Seafoam|GetSeafoam%20Speed) :!class /Script/Engine.KismetMaterialLibrary)
      (Rendering|Material|SetScalarParameterValue "/Game/Ocean/Materials/MPC_Ocean.MPC_Ocean" "SeafoamDistortion" (Variables|Seafoam|GetSeafoam%20Distortion) :!class /Script/Engine.KismetMaterialLibrary)
      (Rendering|Material|SetScalarParameterValue "/Game/Ocean/Materials/MPC_Ocean.MPC_Ocean" "SeafoamHeightPower" (Variables|Seafoam|GetSeafoam%20Height%20Power) :!class /Script/Engine.KismetMaterialLibrary)
      (Rendering|Material|SetScalarParameterValue "/Game/Ocean/Materials/MPC_Ocean.MPC_Ocean" "SeafoamHeightMultiply" (Variables|Seafoam|GetSeafoam%20Height%20Multiply) :!class /Script/Engine.KismetMaterialLibrary)
      ;[1 1 1] Foam Wave Caps
      (Rendering|Material|SetScalarParameterValue "/Game/Ocean/Materials/MPC_Ocean.MPC_Ocean" "FoamCapsOpacity" (Variables|FoamWaveCaps|GetFoam%20Caps%20Opacity) :!class /Script/Engine.KismetMaterialLibrary)
      (Rendering|Material|SetScalarParameterValue "/Game/Ocean/Materials/MPC_Ocean.MPC_Ocean" "FoamCapsHeight" (Variables|FoamWaveCaps|GetFoam%20Caps%20Height) :!class /Script/Engine.KismetMaterialLibrary)
      (Rendering|Material|SetScalarParameterValue "/Game/Ocean/Materials/MPC_Ocean.MPC_Ocean" "FoamCapsPower" (Variables|FoamWaveCaps|GetFoam%20caps%20Power) :!class /Script/Engine.KismetMaterialLibrary)
      ;[1 1 1] Cubemap Reflection
      (Rendering|Material|SetScalarParameterValue "/Game/Ocean/Materials/MPC_Ocean.MPC_Ocean" "CubemapReflectionStrength" (Variables|CubemapReflection|GetCubemap%20Reflection%20Strength) :!class /Script/Engine.KismetMaterialLibrary))
    (:then_7
      (Rendering|Material|SetTextureParameterValue "Wave Normal" 0)
      (Rendering|Material|SetTextureParameterValue "Small Wave Normal" 0)
      (Rendering|Material|SetTextureParameterValue "Far Wave Normal" 0)
      (Rendering|Material|SetTextureParameterValue "Large Wave Height" 0)
      (Rendering|Material|SetTextureParameterValue "ShoreFoam" 0)
      (Rendering|Material|SetTextureParameterValue "ShoreFoam2" 0)
      (Rendering|Material|SetTextureParameterValue "ShoreFoamRoughness" 0)
      (Rendering|Material|SetTextureParameterValue "Seafoam Texture" 0)
      (Rendering|Material|SetTextureParameterValue "Reflection Cubemap" 0))))

(fn SetGlobalParameters
  (bind _wave_clusters (Variables|OceanManager|GetWave%20Clusters))
  (bind _heightmaptexture (Variables|OceanManager|GetHeightmapTexture))
  (bind _landscape (Variables|OceanManager|Getlandscape))
  (bind _item (Utilities|Array|Get(acopy) _wave_clusters))
  (bind (_rotation _length _amplitude _steepness _timemultiplier) (Utilities|Struct|BreakWaveParameters _item))
  (Utilities|FlowControl|Sequence
    (:then_0
      (if (> (Utilities|Array|Length (Variables|OceanManager|GetWave%20Clusters)) 0)
        ;[1 1 1] Wave Set Properties
        (Rendering|Material|SetVectorParameterValue "/Game/Ocean/Materials/MPC_Ocean.MPC_Ocean" "WavesDirectionV2" (Utilities|Struct|MakeLinearColor (Variables|OceanManager|GetGlobal%20Wave%20Direction) (Variables|OceanManager|GetGlobal%20Wave%20Direction) 0.0 0.0) :!class /Script/Engine.KismetMaterialLibrary)
        (Rendering|Material|SetScalarParameterValue "/Game/Ocean/Materials/MPC_Ocean.MPC_Ocean" "WaveSetRotation" _rotation :!class /Script/Engine.KismetMaterialLibrary)
        (Rendering|Material|SetScalarParameterValue "/Game/Ocean/Materials/MPC_Ocean.MPC_Ocean" "WaveSetLength" _length :!class /Script/Engine.KismetMaterialLibrary)
        (Rendering|Material|SetScalarParameterValue "/Game/Ocean/Materials/MPC_Ocean.MPC_Ocean" "WaveSetAmplitude" (* _amplitude (Variables|OceanManager|GetGlobalWaveAmplitude)) :!class /Script/Engine.KismetMaterialLibrary)
        (Rendering|Material|SetScalarParameterValue "/Game/Ocean/Materials/MPC_Ocean.MPC_Ocean" "WaveSetSteepness" _steepness :!class /Script/Engine.KismetMaterialLibrary)
        (Rendering|Material|SetScalarParameterValue "/Game/Ocean/Materials/MPC_Ocean.MPC_Ocean" "WaveSetTimeMultiplier" (* _timemultiplier (Variables|OceanManager|GetGlobal%20Wave%20Speed)) :!class /Script/Engine.KismetMaterialLibrary)))
    (:then_1
      (Utilities|IsValid (Variables|OceanManager|Getlandscape)
        (:Is%20Valid
          (Utilities|IsValid _heightmaptexture
            (:Is%20Valid
              (Rendering|Material|SetVectorParameterValue "/Game/Ocean/Materials/MPC_Ocean.MPC_Ocean" "HeightmapSizeXY" (Utilities|Struct|MakeLinearColor (Math|Conversions|ToFloat(Integer) (Class|Texture2D|BlueprintGetSizeX _heightmaptexture)) (Math|Conversions|ToFloat(Integer) (Class|Texture2D|BlueprintGetSizeY _heightmaptexture)) 0.0 0.0) :!class /Script/Engine.KismetMaterialLibrary)
              (Rendering|Material|SetScalarParameterValue "/Game/Ocean/Materials/MPC_Ocean.MPC_Ocean" "ModulationStartHeight" (Variables|OceanManager|GetModulation%20Start%20Height) :!class /Script/Engine.KismetMaterialLibrary)
              (Rendering|Material|SetScalarParameterValue "/Game/Ocean/Materials/MPC_Ocean.MPC_Ocean" "ModulationMaxHeight" (Variables|OceanManager|GetModulation%20Max%20Height) :!class /Script/Engine.KismetMaterialLibrary)
              (Rendering|Material|SetScalarParameterValue "/Game/Ocean/Materials/MPC_Ocean.MPC_Ocean" "ModulationPower" (Variables|OceanManager|GetModulation%20Power) :!class /Script/Engine.KismetMaterialLibrary)
              (Rendering|Material|SetTextureParameterValue (Variables|Default|GetMID_Ocean) "LandHeightmap" (Variables|OceanManager|GetHeightmapTexture))
              (Rendering|Material|SetVectorParameterValue "/Game/Ocean/Materials/MPC_Ocean.MPC_Ocean" "LandscapeLoc" (Math|Conversions|ToLinearColor(Vector) (Transformation|GetActorLocation _landscape)) :!class /Script/Engine.KismetMaterialLibrary)
              (Rendering|Material|SetVectorParameterValue "/Game/Ocean/Materials/MPC_Ocean.MPC_Ocean" "LandscapeScale" (Math|Conversions|ToLinearColor(Vector) (Transformation|GetActorScale3D _landscape)) :!class /Script/Engine.KismetMaterialLibrary))))))))