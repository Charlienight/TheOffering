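; Small pool water actor, in the Old ocean folder, that configures ocean shader materials and waves on its SmallPool component.
; Construction creates dynamic surface and depth instances from the chosen shader type, both on slot 0, so the depth instance replaces the surface one.
; Construction and BeginPlay push eight waves, first-cluster globals, look settings and sea level into shared MPC_Ocean.
; Textures go to the instances, including an optional landscape heightmap for modulation.
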(event EventBeginPlay
  (CallFunction|CreateWaveSet2)
  (CallFunction|SetGlobalParameters2)
  (CallFunction|SetDisplayParameters2))

(fn ConstructionScript
  (bind _small_pool (Variables|Default|GetSmall%20Pool))
  (Utilities|FlowControl|Sequence
    (:then_0
      ;[1 1 1] materiela instance
      (bind _returnvalue (Rendering|Material|CreateDynamicMaterialInstance (Variables|Default|GetSmall%20Pool) 0 (Utilities|Select :Index (Variables|Apperance|GetOceanShader_0) :NewEnumerator0 "/Game/Ocean/Materials/M_Ocean_Versions/M_Ocean_Old.M_Ocean_Old" :NewEnumerator1 "/Game/Ocean/Materials/M_Ocean_Versions/M_Ocean.M_Ocean" :NewEnumerator2 "/Game/Ocean/Materials/M_Ocean_Versions/M_Ocean_SSR.M_Ocean_SSR" :NewEnumerator3 "/Game/Ocean/Materials/M_Ocean_Versions/M_Inst_Ocean_Foam.M_Inst_Ocean_Foam" :NewEnumerator8 "/Game/Ocean/Materials/M_Ocean_Versions/M_Inst_Ocean_Foam_Cubemap.M_Inst_Ocean_Foam_Cubemap" :NewEnumerator6 "/Game/Ocean/Materials/M_Ocean_Versions/M_Inst_Ocean_SSR_Foam.M_Inst_Ocean_SSR_Foam" :NewEnumerator7 "/Game/Ocean/Materials/M_Ocean_Versions/M_Inst_Ocean_SSR_Foam_Cubemap.M_Inst_Ocean_SSR_Foam_Cubemap" :NewEnumerator4 "/Game/Ocean/Materials/M_Ocean_Versions/M_Inst_Ocean_Nogerstner.M_Inst_Ocean_Nogerstner" :NewEnumerator5 "/Game/Ocean/Materials/M_Ocean_Versions/M_Inst_Ocean_SSR_Nogerstner.M_Inst_Ocean_SSR_Nogerstner" :NewEnumerator9 "/Game/Ocean/Materials/M_Ocean_Versions/M_Inst_Ocean_Ultra.M_Inst_Ocean_Ultra" :NewEnumerator10 0) :!class /Script/Engine.PrimitiveComponent))
      (Variables|Default|SetMID_Ocean_0 _returnvalue)
      ;[1 1 1] Setup the material instance
      (switch Utilities|FlowControl|Switch|SwitchonOceanShaderEnum (Variables|Apperance|GetOceanShader_0)
        (:NewEnumerator0
          (bind _returnvalue_2 (Rendering|Material|CreateDynamicMaterialInstance _small_pool 0 "/Game/Ocean/Materials/M_Ocean_Versions/M_Inst_Ocean_Depth.M_Inst_Ocean_Depth" :!class /Script/Engine.PrimitiveComponent :!label _label))
          (bind _output_get (Variables|Default|SetMID_Ocean_Depth_0 _returnvalue_2))
          (Rendering|Material|SetMaterial (Variables|Default|GetSmall%20Pool) 0 _output_get))
        (:NewEnumerator1
          (goto _label))
        (:NewEnumerator2
          (goto _label))
        (:NewEnumerator3
          (goto _label))
        (:NewEnumerator8
          (goto _label))
        (:NewEnumerator6
          (goto _label))
        (:NewEnumerator7
          (goto _label))
        (:NewEnumerator4
          (bind _returnvalue_3 (Rendering|Material|CreateDynamicMaterialInstance _small_pool 0 "/Game/Ocean/Materials/M_Ocean_Versions/M_Inst_Ocean_Depth_Nogerstner.M_Inst_Ocean_Depth_Nogerstner" :!class /Script/Engine.PrimitiveComponent :!label _label_2))
          (Variables|Default|SetMID_Ocean_Depth_0 _returnvalue_3))
        (:NewEnumerator5
          (goto _label_2))
        (:NewEnumerator9
          (bind _returnvalue_4 (Rendering|Material|CreateDynamicMaterialInstance _small_pool 0 "/Game/Ocean/Materials/M_Ocean_Versions/M_Inst_Ocean_Ultra.M_Inst_Ocean_Ultra" :!class /Script/Engine.PrimitiveComponent))
          (Variables|Default|SetMID_Ocean_Depth_0 _returnvalue_4))
        (:NewEnumerator10
          (goto _label))))
    (:then_1
      ;[1 1 1] Set global parameters
      (CallFunction|SetGlobalParameters2)
      (CallFunction|SetDisplayParameters2))
    (:then_2
      ;[1 1 1] Create wave set
      (CallFunction|CreateWaveSet2))))

(fn CreateWaveSet2
  ;[1 1 1] Intiliaze Wave Set
  (Utilities|FlowControl|Sequence
    (:then_0
      (if (> (Utilities|Array|Length (Variables|OceanManager|GetWaveSetOffsetsOverride_0)) 0)
        (LocalVariables|SetSetPharams (Utilities|Array|Get(acopy) (Variables|OceanManager|GetWaveSetOffsetsOverride_0)))))
    (:then_1
      (Rendering|Material|SetVectorParameterValue "/Game/Ocean/Materials/MPC_Ocean.MPC_Ocean" "Set01Wave01" (Math|Color|MakeColor (.Rotation (Utilities|Struct|BreakWaveParameters (.Wave01 (Utilities|Struct|BreakWaveSet (LocalVariables|GetSetPharams))))) (.Length (Utilities|Struct|BreakWaveParameters (.Wave01 (Utilities|Struct|BreakWaveSet (LocalVariables|GetSetPharams))))) (.Amplitude (Utilities|Struct|BreakWaveParameters (.Wave01 (Utilities|Struct|BreakWaveSet (LocalVariables|GetSetPharams))))) (.Steepness (Utilities|Struct|BreakWaveParameters (.Wave01 (Utilities|Struct|BreakWaveSet (LocalVariables|GetSetPharams)))))) :!class /Script/Engine.KismetMaterialLibrary)
      (Rendering|Material|SetVectorParameterValue "/Game/Ocean/Materials/MPC_Ocean.MPC_Ocean" "Set01Wave02" (Math|Color|MakeColor (.Rotation (Utilities|Struct|BreakWaveParameters (.Wave02 (Utilities|Struct|BreakWaveSet (LocalVariables|GetSetPharams))))) (.Length (Utilities|Struct|BreakWaveParameters (.Wave02 (Utilities|Struct|BreakWaveSet (LocalVariables|GetSetPharams))))) (.Amplitude (Utilities|Struct|BreakWaveParameters (.Wave02 (Utilities|Struct|BreakWaveSet (LocalVariables|GetSetPharams))))) (.Steepness (Utilities|Struct|BreakWaveParameters (.Wave02 (Utilities|Struct|BreakWaveSet (LocalVariables|GetSetPharams)))))) :!class /Script/Engine.KismetMaterialLibrary)
      (Rendering|Material|SetVectorParameterValue "/Game/Ocean/Materials/MPC_Ocean.MPC_Ocean" "Set01Wave03" (Math|Color|MakeColor (.Rotation (Utilities|Struct|BreakWaveParameters (.Wave03 (Utilities|Struct|BreakWaveSet (LocalVariables|GetSetPharams))))) (.Length (Utilities|Struct|BreakWaveParameters (.Wave03 (Utilities|Struct|BreakWaveSet (LocalVariables|GetSetPharams))))) (.Amplitude (Utilities|Struct|BreakWaveParameters (.Wave03 (Utilities|Struct|BreakWaveSet (LocalVariables|GetSetPharams))))) (.Steepness (Utilities|Struct|BreakWaveParameters (.Wave03 (Utilities|Struct|BreakWaveSet (LocalVariables|GetSetPharams)))))) :!class /Script/Engine.KismetMaterialLibrary)
      (Rendering|Material|SetVectorParameterValue "/Game/Ocean/Materials/MPC_Ocean.MPC_Ocean" "Set01Wave04" (Math|Color|MakeColor (.Rotation (Utilities|Struct|BreakWaveParameters (.Wave04 (Utilities|Struct|BreakWaveSet (LocalVariables|GetSetPharams))))) (.Length (Utilities|Struct|BreakWaveParameters (.Wave04 (Utilities|Struct|BreakWaveSet (LocalVariables|GetSetPharams))))) (.Amplitude (Utilities|Struct|BreakWaveParameters (.Wave04 (Utilities|Struct|BreakWaveSet (LocalVariables|GetSetPharams))))) (.Steepness (Utilities|Struct|BreakWaveParameters (.Wave04 (Utilities|Struct|BreakWaveSet (LocalVariables|GetSetPharams)))))) :!class /Script/Engine.KismetMaterialLibrary)
      (Rendering|Material|SetVectorParameterValue "/Game/Ocean/Materials/MPC_Ocean.MPC_Ocean" "Set01Wave05" (Math|Color|MakeColor (.Rotation (Utilities|Struct|BreakWaveParameters (.Wave05 (Utilities|Struct|BreakWaveSet (LocalVariables|GetSetPharams))))) (.Length (Utilities|Struct|BreakWaveParameters (.Wave05 (Utilities|Struct|BreakWaveSet (LocalVariables|GetSetPharams))))) (.Amplitude (Utilities|Struct|BreakWaveParameters (.Wave05 (Utilities|Struct|BreakWaveSet (LocalVariables|GetSetPharams))))) (.Steepness (Utilities|Struct|BreakWaveParameters (.Wave05 (Utilities|Struct|BreakWaveSet (LocalVariables|GetSetPharams)))))) :!class /Script/Engine.KismetMaterialLibrary)
      (Rendering|Material|SetVectorParameterValue "/Game/Ocean/Materials/MPC_Ocean.MPC_Ocean" "Set01Wave06" (Math|Color|MakeColor (.Rotation (Utilities|Struct|BreakWaveParameters (.Wave06 (Utilities|Struct|BreakWaveSet (LocalVariables|GetSetPharams))))) (.Length (Utilities|Struct|BreakWaveParameters (.Wave06 (Utilities|Struct|BreakWaveSet (LocalVariables|GetSetPharams))))) (.Amplitude (Utilities|Struct|BreakWaveParameters (.Wave06 (Utilities|Struct|BreakWaveSet (LocalVariables|GetSetPharams))))) (.Steepness (Utilities|Struct|BreakWaveParameters (.Wave06 (Utilities|Struct|BreakWaveSet (LocalVariables|GetSetPharams)))))) :!class /Script/Engine.KismetMaterialLibrary)
      (Rendering|Material|SetVectorParameterValue "/Game/Ocean/Materials/MPC_Ocean.MPC_Ocean" "Set01Wave07" (Math|Color|MakeColor (.Rotation (Utilities|Struct|BreakWaveParameters (.Wave07 (Utilities|Struct|BreakWaveSet (LocalVariables|GetSetPharams))))) (.Length (Utilities|Struct|BreakWaveParameters (.Wave07 (Utilities|Struct|BreakWaveSet (LocalVariables|GetSetPharams))))) (.Amplitude (Utilities|Struct|BreakWaveParameters (.Wave07 (Utilities|Struct|BreakWaveSet (LocalVariables|GetSetPharams))))) (.Steepness (Utilities|Struct|BreakWaveParameters (.Wave07 (Utilities|Struct|BreakWaveSet (LocalVariables|GetSetPharams)))))) :!class /Script/Engine.KismetMaterialLibrary)
      (Rendering|Material|SetVectorParameterValue "/Game/Ocean/Materials/MPC_Ocean.MPC_Ocean" "Set01Wave08" (Math|Color|MakeColor (.Rotation (Utilities|Struct|BreakWaveParameters (.Wave08 (Utilities|Struct|BreakWaveSet (LocalVariables|GetSetPharams))))) (.Length (Utilities|Struct|BreakWaveParameters (.Wave08 (Utilities|Struct|BreakWaveSet (LocalVariables|GetSetPharams))))) (.Amplitude (Utilities|Struct|BreakWaveParameters (.Wave08 (Utilities|Struct|BreakWaveSet (LocalVariables|GetSetPharams))))) (.Steepness (Utilities|Struct|BreakWaveParameters (.Wave08 (Utilities|Struct|BreakWaveSet (LocalVariables|GetSetPharams)))))) :!class /Script/Engine.KismetMaterialLibrary))))

(fn SetDisplayParameters2
  (bind _mid_ocean_0 (Variables|Default|GetMID_Ocean_0))
  (Utilities|FlowControl|Sequence
    (:then_0
      ;[1 1 1] Base Material Props
      (Rendering|Material|SetVectorParameterValue "/Game/Ocean/Materials/MPC_Ocean.MPC_Ocean" "BaseColorDark" (Variables|Apperance|GetBase%20Color%20Dark_0) :!class /Script/Engine.KismetMaterialLibrary)
      (Rendering|Material|SetVectorParameterValue "/Game/Ocean/Materials/MPC_Ocean.MPC_Ocean" "BaseColorLight" (Variables|Apperance|GetBase%20Color%20Light_0) :!class /Script/Engine.KismetMaterialLibrary)
      (Rendering|Material|SetScalarParameterValue "/Game/Ocean/Materials/MPC_Ocean.MPC_Ocean" "BaseColorLerp" (Variables|Apperance|GetBase%20Color%20Lerp_0) :!class /Script/Engine.KismetMaterialLibrary)
      (Rendering|Material|SetScalarParameterValue "/Game/Ocean/Materials/MPC_Ocean.MPC_Ocean" "BaseFresnelPower" (Variables|Apperance|GetFresnel%20Power_0) :!class /Script/Engine.KismetMaterialLibrary)
      (Rendering|Material|SetScalarParameterValue "/Game/Ocean/Materials/MPC_Ocean.MPC_Ocean" "BaseFresnelReflect" (Variables|Apperance|GetBase%20Fresnel%20Reflect_0) :!class /Script/Engine.KismetMaterialLibrary)
      (Rendering|Material|SetScalarParameterValue "/Game/Ocean/Materials/MPC_Ocean.MPC_Ocean" "Metallic" (Variables|Apperance|GetMetallic_0) :!class /Script/Engine.KismetMaterialLibrary)
      (Rendering|Material|SetScalarParameterValue "/Game/Ocean/Materials/MPC_Ocean.MPC_Ocean" "Roughness" (Variables|Apperance|GetRoughness_0) :!class /Script/Engine.KismetMaterialLibrary)
      (Rendering|Material|SetScalarParameterValue "/Game/Ocean/Materials/MPC_Ocean.MPC_Ocean" "Specular" (Variables|Apperance|GetSpecular_0) :!class /Script/Engine.KismetMaterialLibrary)
      (Rendering|Material|SetScalarParameterValue "/Game/Ocean/Materials/MPC_Ocean.MPC_Ocean" "TesselationMultiplier" (Variables|Apperance|GetTesselation%20Multiplier) :!class /Script/Engine.KismetMaterialLibrary)
      (Rendering|Material|SetVectorParameterValue "/Game/Ocean/Materials/MPC_Ocean.MPC_Ocean" "ShallowColor" (Variables|Apperance|GetShallow%20Water%20Color_0) :!class /Script/Engine.KismetMaterialLibrary))
    (:then_1
      ;[1 1 1] Base Extended Props
      (Rendering|Material|SetScalarParameterValue "/Game/Ocean/Materials/MPC_Ocean.MPC_Ocean" "Opacity" (Variables|Apperance|GetOpacity_0) :!class /Script/Engine.KismetMaterialLibrary)
      (Rendering|Material|SetScalarParameterValue "/Game/Ocean/Materials/MPC_Ocean.MPC_Ocean" "DepthFade" (Variables|Apperance|GetBase%20Depth%20Fade_0) :!class /Script/Engine.KismetMaterialLibrary)
      (Rendering|Material|SetScalarParameterValue "/Game/Ocean/Materials/MPC_Ocean.MPC_Ocean" "DistortionStrength" (Variables|Apperance|GetDistortion%20Strength_0) :!class /Script/Engine.KismetMaterialLibrary)
      (Rendering|Material|SetScalarParameterValue "/Game/Ocean/Materials/MPC_Ocean.MPC_Ocean" "SceneColorDepthFade" (Variables|Apperance|GetScene%20Color%20Custom%20Depth_0) :!class /Script/Engine.KismetMaterialLibrary)
      (Rendering|Material|SetScalarParameterValue "/Game/Ocean/Materials/MPC_Ocean.MPC_Ocean" "FoamScale" (Variables|Apperance|GetFoam%20scale_0) :!class /Script/Engine.KismetMaterialLibrary)
      (Rendering|Material|SetScalarParameterValue "/Game/Ocean/Materials/MPC_Ocean.MPC_Ocean" "DepthTest1" (Variables|Apperance|GetFoam%20Depth%201_0) :!class /Script/Engine.KismetMaterialLibrary)
      (Rendering|Material|SetScalarParameterValue "/Game/Ocean/Materials/MPC_Ocean.MPC_Ocean" "DepthTest2" (Variables|Apperance|GetFoam%20Depth%202_0) :!class /Script/Engine.KismetMaterialLibrary)
      (Rendering|Material|SetScalarParameterValue "/Game/Ocean/Materials/MPC_Ocean.MPC_Ocean" "FoamTimeScale" (Variables|Apperance|GetFoam%20Time%20Scale_0) :!class /Script/Engine.KismetMaterialLibrary)
      (Rendering|Material|SetScalarParameterValue "/Game/Ocean/Materials/MPC_Ocean.MPC_Ocean" "FoamSoftness" (Variables|Apperance|GetFoam%20Softness%201_0) :!class /Script/Engine.KismetMaterialLibrary)
      (Rendering|Material|SetScalarParameterValue "/Game/Ocean/Materials/MPC_Ocean.MPC_Ocean" "SceneDepthSoftness" (Variables|Apperance|GetScene%20Depth%20Softness_0) :!class /Script/Engine.KismetMaterialLibrary)
      (Rendering|Material|SetScalarParameterValue "/Game/Ocean/Materials/MPC_Ocean.MPC_Ocean" "BaseDepthFadeSoftness" (Variables|Apperance|GetBase%20Depth%20Fade%20Softness) :!class /Script/Engine.KismetMaterialLibrary))
    (:then_2
      ;[1 1 1] Subsurface Scattering
      (Rendering|Material|SetVectorParameterValue "/Game/Ocean/Materials/MPC_Ocean.MPC_Ocean" "SSS_Color" (Variables|SubsurafeceScattering|GetSSS_Color_0) :!class /Script/Engine.KismetMaterialLibrary)
      (Rendering|Material|SetScalarParameterValue "/Game/Ocean/Materials/MPC_Ocean.MPC_Ocean" "SSS_Scale" (Variables|SubsurafeceScattering|GetSSS_Scale) :!class /Script/Engine.KismetMaterialLibrary)
      (Rendering|Material|SetScalarParameterValue "/Game/Ocean/Materials/MPC_Ocean.MPC_Ocean" "SSS_Intensity" (Variables|SubsurafeceScattering|GetSSS_Intensity_0) :!class /Script/Engine.KismetMaterialLibrary)
      (Rendering|Material|SetScalarParameterValue "/Game/Ocean/Materials/MPC_Ocean.MPC_Ocean" "SSS_LightDepth" (Variables|SubsurafeceScattering|GetSSS_LightDepth_0) :!class /Script/Engine.KismetMaterialLibrary)
      (Rendering|Material|SetScalarParameterValue "/Game/Ocean/Materials/MPC_Ocean.MPC_Ocean" "SSS_MacroNormalStrength" (Variables|SubsurafeceScattering|GetSSS_Macro%20Normal%20Strength) :!class /Script/Engine.KismetMaterialLibrary))
    (:then_3
      ;[1 1 1] Panning Normals
      (Rendering|Material|SetScalarParameterValue "/Game/Ocean/Materials/MPC_Ocean.MPC_Ocean" "PanWaveLerp" (Variables|PanningNormals|GetPan%20Wave%20Lerp_0) :!class /Script/Engine.KismetMaterialLibrary)
      (Rendering|Material|SetScalarParameterValue "/Game/Ocean/Materials/MPC_Ocean.MPC_Ocean" "PanWaveIntensity" (Variables|PanningNormals|GetPan%20Wave%20Intensity_0) :!class /Script/Engine.KismetMaterialLibrary)
      (Rendering|Material|SetScalarParameterValue "/Game/Ocean/Materials/MPC_Ocean.MPC_Ocean" "PanWaveTimeScale" (Variables|PanningNormals|GetPan%20Wave%20Time%20Scale_0) :!class /Script/Engine.KismetMaterialLibrary)
      (Rendering|Material|SetScalarParameterValue "/Game/Ocean/Materials/MPC_Ocean.MPC_Ocean" "PanWaveSize" (Variables|PanningNormals|GetPan%20Wave%20Size_0) :!class /Script/Engine.KismetMaterialLibrary)
      (Rendering|Material|SetVectorParameterValue "/Game/Ocean/Materials/MPC_Ocean.MPC_Ocean" "PanWave01SpeedV2" (Math|Conversions|ToLinearColor(Vector) (Variables|PanningNormals|GetPanner%2001%20Speed_0)) :!class /Script/Engine.KismetMaterialLibrary)
      (Rendering|Material|SetVectorParameterValue "/Game/Ocean/Materials/MPC_Ocean.MPC_Ocean" "PanWave01SpeedV2" (Math|Conversions|ToLinearColor(Vector) (Variables|PanningNormals|GetPanner%2002%20Speed_0)) :!class /Script/Engine.KismetMaterialLibrary)
      (Rendering|Material|SetVectorParameterValue "/Game/Ocean/Materials/MPC_Ocean.MPC_Ocean" "PanWave01SpeedV2" (Math|Conversions|ToLinearColor(Vector) (Variables|PanningNormals|GetPanner%2003%20Speed_0)) :!class /Script/Engine.KismetMaterialLibrary)
      ;[1 1 1] Macro Waves
      (Rendering|Material|SetScalarParameterValue "/Game/Ocean/Materials/MPC_Ocean.MPC_Ocean" "MacroScale" (Variables|PanningNormals|GetMacro%20Wave%20Scale_0) :!class /Script/Engine.KismetMaterialLibrary)
      (Rendering|Material|SetScalarParameterValue "/Game/Ocean/Materials/MPC_Ocean.MPC_Ocean" "MacroSpeed" (Variables|PanningNormals|GetMacro%20Wave%20speed_0) :!class /Script/Engine.KismetMaterialLibrary)
      (Rendering|Material|SetScalarParameterValue "/Game/Ocean/Materials/MPC_Ocean.MPC_Ocean" "MacroAmplify" (Variables|PanningNormals|GetMacro%20Wave%20Amplitude) :!class /Script/Engine.KismetMaterialLibrary))
    (:then_4
      ;[1 1 1] Detail, Medium and Fr Normals
      (Rendering|Material|SetScalarParameterValue "/Game/Ocean/Materials/MPC_Ocean.MPC_Ocean" "DetailNormalScale" (Variables|Detail,Mediumandfarnormals|GetDetail%20Normal%20Scale_0) :!class /Script/Engine.KismetMaterialLibrary)
      (Rendering|Material|SetScalarParameterValue "/Game/Ocean/Materials/MPC_Ocean.MPC_Ocean" "DetailNormalSpeed" (Variables|Detail,Mediumandfarnormals|GetDetail%20Normal%20Speed_0) :!class /Script/Engine.KismetMaterialLibrary)
      (Rendering|Material|SetScalarParameterValue "/Game/Ocean/Materials/MPC_Ocean.MPC_Ocean" "DetailNormalStrength" (Variables|Detail,Mediumandfarnormals|GetDetail%20Normal%20Strength_0) :!class /Script/Engine.KismetMaterialLibrary)
      (Rendering|Material|SetScalarParameterValue "/Game/Ocean/Materials/MPC_Ocean.MPC_Ocean" "MediumNormalScale" (Variables|Detail,Mediumandfarnormals|GetMedium%20Normal%20Scale_0) :!class /Script/Engine.KismetMaterialLibrary)
      (Rendering|Material|SetScalarParameterValue "/Game/Ocean/Materials/MPC_Ocean.MPC_Ocean" "MediumNormalSpeed" (Variables|Detail,Mediumandfarnormals|GetMedium%20Normal%20Speed_0) :!class /Script/Engine.KismetMaterialLibrary)
      (Rendering|Material|SetScalarParameterValue "/Game/Ocean/Materials/MPC_Ocean.MPC_Ocean" "MediumNormalStrength" (Variables|Detail,Mediumandfarnormals|GetMedium%20Normal%20Strength_0) :!class /Script/Engine.KismetMaterialLibrary)
      (Rendering|Material|SetScalarParameterValue "/Game/Ocean/Materials/MPC_Ocean.MPC_Ocean" "FarNormalScale" (Variables|Detail,Mediumandfarnormals|GetFar%20Normal%20Scale_0) :!class /Script/Engine.KismetMaterialLibrary)
      (Rendering|Material|SetScalarParameterValue "/Game/Ocean/Materials/MPC_Ocean.MPC_Ocean" "FarNormalSpeed" (Variables|Detail,Mediumandfarnormals|GetFar%20Normal%20Speed_0) :!class /Script/Engine.KismetMaterialLibrary)
      (Rendering|Material|SetScalarParameterValue "/Game/Ocean/Materials/MPC_Ocean.MPC_Ocean" "FarNormalStrength" (Variables|Detail,Mediumandfarnormals|GetFar%20Normal%20Strength_0) :!class /Script/Engine.KismetMaterialLibrary)
      (Rendering|Material|SetScalarParameterValue "/Game/Ocean/Materials/MPC_Ocean.MPC_Ocean" "FarNormalBlendDistance" (Variables|Detail,Mediumandfarnormals|GetFar%20Normal%20Blend%20Distance_0) :!class /Script/Engine.KismetMaterialLibrary)
      (Rendering|Material|SetScalarParameterValue "/Game/Ocean/Materials/MPC_Ocean.MPC_Ocean" "FarNormalBlendFalloff" (Variables|Detail,Mediumandfarnormals|GetFar%20Normal%20Blend%20Falloff_0) :!class /Script/Engine.KismetMaterialLibrary))
    (:then_5
      ;[1 1 1] Heightmap
      (Rendering|Material|SetScalarParameterValue "/Game/Ocean/Materials/MPC_Ocean.MPC_Ocean" "HeightmapDisplacement" (Variables|Heightmap|GetHeightmap%20Displacement_0) :!class /Script/Engine.KismetMaterialLibrary)
      (Rendering|Material|SetScalarParameterValue "/Game/Ocean/Materials/MPC_Ocean.MPC_Ocean" "HeightmapScale" (Variables|Heightmap|GetHeightMap%20Scale_0) :!class /Script/Engine.KismetMaterialLibrary)
      (Rendering|Material|SetScalarParameterValue "/Game/Ocean/Materials/MPC_Ocean.MPC_Ocean" "HeightmapSpeed" (Variables|Heightmap|GetHeightmap%20Speed_0) :!class /Script/Engine.KismetMaterialLibrary))
    (:then_6
      ;[1 1 1] Seafoam parameters
      (Rendering|Material|SetScalarParameterValue "/Game/Ocean/Materials/MPC_Ocean.MPC_Ocean" "SeafoamScale" (Variables|Seafoam|GetSeafoam%20Scale_0) :!class /Script/Engine.KismetMaterialLibrary)
      (Rendering|Material|SetScalarParameterValue "/Game/Ocean/Materials/MPC_Ocean.MPC_Ocean" "SeafoamSpeed" (Variables|Seafoam|GetSeafoam%20Speed_0) :!class /Script/Engine.KismetMaterialLibrary)
      (Rendering|Material|SetScalarParameterValue "/Game/Ocean/Materials/MPC_Ocean.MPC_Ocean" "SeafoamDistortion" (Variables|Seafoam|GetSeafoam%20Distortion_0) :!class /Script/Engine.KismetMaterialLibrary)
      (Rendering|Material|SetScalarParameterValue "/Game/Ocean/Materials/MPC_Ocean.MPC_Ocean" "SeafoamHeightPower" (Variables|Seafoam|GetSeafoam%20Hieght%20Power) :!class /Script/Engine.KismetMaterialLibrary)
      (Rendering|Material|SetScalarParameterValue "/Game/Ocean/Materials/MPC_Ocean.MPC_Ocean" "SeafoamHeightMultiply" (Variables|Seafoam|GetSeafoam%20Hieght%20Multiply) :!class /Script/Engine.KismetMaterialLibrary)
      ;[1 1 1] Foam Wave Caps
      (Rendering|Material|SetScalarParameterValue "/Game/Ocean/Materials/MPC_Ocean.MPC_Ocean" "FoamCapsOpacity" (Variables|FoamWavecaps|GetFoam%20Caps%20Opcaity) :!class /Script/Engine.KismetMaterialLibrary)
      (Rendering|Material|SetScalarParameterValue "/Game/Ocean/Materials/MPC_Ocean.MPC_Ocean" "FoamCapsHeight" (Variables|FoamWavecaps|GetFoam%20caps%20height_0) :!class /Script/Engine.KismetMaterialLibrary)
      (Rendering|Material|SetScalarParameterValue "/Game/Ocean/Materials/MPC_Ocean.MPC_Ocean" "FoamCapsPower" (Variables|FoamWavecaps|GetFoam%20caps%20Power_0) :!class /Script/Engine.KismetMaterialLibrary)
      ;[1 1 1] Cubemap reflection
      (Rendering|Material|SetScalarParameterValue "/Game/Ocean/Materials/MPC_Ocean.MPC_Ocean" "CubemapReflectionStrength" (Variables|CubemapReflection|GetCubemap%20Reflection%20Strength_0) :!class /Script/Engine.KismetMaterialLibrary))
    (:then_7
      ;[1 1 1] Texture paramters
      (Rendering|Material|SetTextureParameterValue _mid_ocean_0 "Wave Normal" (Variables|Textures|GetMedium%20Wave%20Normal_0))
      (Rendering|Material|SetTextureParameterValue _mid_ocean_0 "Small Wave Normal" (Variables|Textures|GetSmall%20Wave%20Normal_0))
      (Rendering|Material|SetTextureParameterValue _mid_ocean_0 "Far Wave Normal" (Variables|Textures|GetFar%20Wave%20Normal_0))
      (Rendering|Material|SetTextureParameterValue _mid_ocean_0 "Large Wave Height" (Variables|Textures|GetHeightmap_0))
      (Rendering|Material|SetTextureParameterValue _mid_ocean_0 "ShoreFoam" (Variables|Textures|GetShorefoam_0))
      (Rendering|Material|SetTextureParameterValue _mid_ocean_0 "ShoreFoam2" (Variables|Textures|GetShore%20Foam%202_0))
      (Rendering|Material|SetTextureParameterValue _mid_ocean_0 "ShoreFoamRoughness" (Variables|Textures|GetShore%20Foam%20roughness_0))
      (Rendering|Material|SetTextureParameterValue _mid_ocean_0 "Seafoam Texture" (Variables|Textures|GetSeafoam_0))
      (Rendering|Material|SetTextureParameterValue _mid_ocean_0 "Reflection Cubemap" (Variables|Textures|GetReflkection%20Cubemap)))
    (:then_9
      (Rendering|Material|SetScalarParameterValue "/Game/Ocean/Materials/MPC_Ocean.MPC_Ocean" "SeaLevel" (.z (Transformation|GetWorldLocation (Variables|Default|GetSmall%20Pool))) :!class /Script/Engine.KismetMaterialLibrary))))

(fn SetGlobalParameters2
  (bind _wave_clusters_0 (Variables|OceanManager|GetWave%20Clusters_0))
  (bind _heightmap_texture (Variables|OceanManager|Getheightmap%20texture))
  (bind _item (Utilities|Array|Get(acopy) _wave_clusters_0))
  (bind (_rotation _length _amplitude _steepness _timemultiplier) (Utilities|Struct|BreakWaveParameters _item))
  (Utilities|FlowControl|Sequence
    (:then_0
      ;[1 1 1] Wave Set Prop
      (if (> (Utilities|Array|Length (Variables|OceanManager|GetWave%20Clusters_0)) 0)
        (Rendering|Material|SetVectorParameterValue "/Game/Ocean/Materials/MPC_Ocean.MPC_Ocean" "WavesDirectionV2" (Utilities|Struct|MakeLinearColor (Variables|OceanManager|GetGlobal%20wave%20direction_0) (Variables|OceanManager|GetGlobal%20wave%20direction_0) 0.0 0.0) :!class /Script/Engine.KismetMaterialLibrary)
        (Rendering|Material|SetScalarParameterValue "/Game/Ocean/Materials/MPC_Ocean.MPC_Ocean" "WaveSetRotation" _rotation :!class /Script/Engine.KismetMaterialLibrary)
        (Rendering|Material|SetScalarParameterValue "/Game/Ocean/Materials/MPC_Ocean.MPC_Ocean" "WaveSetLength" _length :!class /Script/Engine.KismetMaterialLibrary)
        (Rendering|Material|SetScalarParameterValue "/Game/Ocean/Materials/MPC_Ocean.MPC_Ocean" "WaveSetAmplitude" (* _amplitude (Variables|OceanManager|GetGlobal%20Wave%20Amplitude)) :!class /Script/Engine.KismetMaterialLibrary)
        (Rendering|Material|SetScalarParameterValue "/Game/Ocean/Materials/MPC_Ocean.MPC_Ocean" "WaveSetSteepness" _steepness :!class /Script/Engine.KismetMaterialLibrary)
        (Rendering|Material|SetScalarParameterValue "/Game/Ocean/Materials/MPC_Ocean.MPC_Ocean" "WaveSetTimeMultiplier" (* _timemultiplier (Variables|OceanManager|GetGlobal%20Wave%20Speed_0)) :!class /Script/Engine.KismetMaterialLibrary)))
    (:then_1
      (Utilities|IsValid (Variables|OceanManager|GetLandscape_0)
        (:Is%20Valid
          (Utilities|IsValid _heightmap_texture
            (:Is%20Valid
              (Rendering|Material|SetVectorParameterValue "/Game/Ocean/Materials/MPC_Ocean.MPC_Ocean" "HeightmapSizeXY" (Utilities|Struct|MakeLinearColor (Math|Conversions|ToFloat(Integer) (Class|Texture2D|BlueprintGetSizeX _heightmap_texture)) (Math|Conversions|ToFloat(Integer) (Class|Texture2D|BlueprintGetSizeY _heightmap_texture)) 0.0 0.0) :!class /Script/Engine.KismetMaterialLibrary)
              (Rendering|Material|SetScalarParameterValue "/Game/Ocean/Materials/MPC_Ocean.MPC_Ocean" "ModulationStartHeight" (Variables|OceanManager|GetModulation%20Start%20Height_0) :!class /Script/Engine.KismetMaterialLibrary)
              (Rendering|Material|SetScalarParameterValue "/Game/Ocean/Materials/MPC_Ocean.MPC_Ocean" "ModulationMaxHeight" (Variables|OceanManager|GetModulation%20Max%20height_0) :!class /Script/Engine.KismetMaterialLibrary)
              (Rendering|Material|SetScalarParameterValue "/Game/Ocean/Materials/MPC_Ocean.MPC_Ocean" "ModulationPower" (Variables|OceanManager|GetModulation%20Power_0) :!class /Script/Engine.KismetMaterialLibrary)
              (Rendering|Material|SetTextureParameterValue (Variables|Default|GetMID_Ocean_0) "LandHeightmap" (Variables|OceanManager|Getheightmap%20texture))
              (Rendering|Material|SetVectorParameterValue "/Game/Ocean/Materials/MPC_Ocean.MPC_Ocean" "LandscapeLoc" (Math|Conversions|ToLinearColor(Vector) (Transformation|GetActorLocation)) :!class /Script/Engine.KismetMaterialLibrary)
              (Rendering|Material|SetVectorParameterValue "/Game/Ocean/Materials/MPC_Ocean.MPC_Ocean" "LandscapeScale" (Math|Conversions|ToLinearColor(Vector) (Transformation|GetActorScale3D)) :!class /Script/Engine.KismetMaterialLibrary))))))))